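; BP_InventoryPickup is a sprite-based world item that the player collects into their inventory.
; Overlapping its Box with the player character enables input on the pickup and swaps to a highlight sprite; leaving disables input and restores the standard sprite.
; Pressing Interact passes InventoryClass to the PaperPlayer's GetItem, then destroys the pickup.
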(event `self.EndFocus`
  (`PaperSpriteComponent.SetSprite` (`self.RenderComponent`) (`self.StandardSprite`)))

(event `self.BeginFocus`
  (`PaperSpriteComponent.SetSprite` (`self.RenderComponent`) (`self.HighlightSprite`)))

(event `InputAction|Interact`
  (params (Key :type "Key Structure" :default "AnyKey"))
  (:`Pressed`
    (bind _aspaper_player (cast `/Game/Veil/Player/PaperPlayer` (`GameplayStatics.GetPlayerCharacter` 0)))
    (`/Game/Veil/Player/PaperPlayer.GetItem` _aspaper_player (`self.InventoryClass`))
    (`self.K2_DestroyActor`)))

(event `self.Box.OnComponentBeginOverlap`
  (params (OverlappedComponent :type "PrimitiveComponent Object Reference") (OtherActor :type "Actor Object Reference") (OtherComp :type "PrimitiveComponent Object Reference") (OtherBodyIndex :type Integer) (bFromSweep :type Boolean) (SweepResult :type "HitResult Structure (by ref)"))
  (if (== OtherActor (`GameplayStatics.GetPlayerCharacter` 0))
    (`self.EnableInput` (`GameplayStatics.GetPlayerController` 0))
    (`self.BeginFocus`)))

(event `self.Box.OnComponentEndOverlap`
  (params (OverlappedComponent :type "PrimitiveComponent Object Reference") (OtherActor :type "Actor Object Reference") (OtherComp :type "PrimitiveComponent Object Reference") (OtherBodyIndex :type Integer))
  (if (== OtherActor (`GameplayStatics.GetPlayerCharacter` 0))
    (`self.DisableInput` (`GameplayStatics.GetPlayerController` 0))
    (`self.EndFocus`)))

(fn `UserConstructionScript`
  (`parent.UserConstructionScript`))